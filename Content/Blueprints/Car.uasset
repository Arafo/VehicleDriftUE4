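; Car is a drivable vehicle Blueprint that the player controls through input axes.
; Forward and Right axis events pass their values straight to the vehicle movement component as throttle and steering.
; The BackCamera axis acts as a look-behind toggle, moving and rotating the camera to face rearward while fully held and restoring its default relative transform otherwise.
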(event `self.ReceiveBeginPlay`)

(event `self.ReceiveActorBeginOverlap`
  (params (OtherActor :type "Actor Object Reference")))

(event `self.ReceiveTick`
  (params (DeltaSeconds :type "Float (single-precision)")))

(event `InputAxis|Forward`
  (params (AxisValue :type "Float (single-precision)"))
  (`WheeledVehicleMovementComponent.SetThrottleInput` (`self.VehicleMovement`) AxisValue))

(event `InputAxis|Right`
  (params (AxisValue :type "Float (single-precision)"))
  (`WheeledVehicleMovementComponent.SetSteeringInput` (`self.VehicleMovement`) AxisValue))

(event `InputAxis|BackCamera`
  (params (AxisValue :type "Float (single-precision)"))
  (bind _returnvalue (>= AxisValue 1.0))
  ;[1 1 1] Mirar hacia atrás
  ;;[1 1 1] Cambiar localización de la cámara
  (`SceneComponent.K2_SetRelativeLocation` (`self.Camera`) (`KismetMathLibrary.MakeVector` (select `bool` _returnvalue :`true` 1200.0 :!type "Float (single-precision)") 0.0 (select `bool` _returnvalue :`true` 200.0 :!type "Float (single-precision)")) false)
  ;;[1 1 1] Cambiar rotación de la cámara
  (`SceneComponent.K2_SetRelativeRotation` (`self.Camera`) (`KismetMathLibrary.MakeRot` (select `bool` _returnvalue :`true` -20.0 :!type "Float (single-precision)") (select `bool` _returnvalue :`true` 180.0 :!type "Float (single-precision)")) false))

(fn `UserConstructionScript`)